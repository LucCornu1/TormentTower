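; MyHordePaperCharacter is a horde character, likely an enemy, that deals contact damage to the player.
; Box overlap with a BP_Player stores that actor and sets CanDamage, while other actors trigger a debug "Hello" print.
; While CanDamage is set, Tick applies damage to the stored player every frame, independent of delta time.
; End overlap also sets CanDamage true, so damage continues after the player leaves the box.
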(event `self.ReceiveTick`
  (params (DeltaSeconds :type "Float (single-precision)"))
  (if (`self.bCanDamage`)
    (`GameplayStatics.ApplyDamage` (`self.PlayerCharacter`) 1.0)))

(event `self.Box.OnComponentBeginOverlap`
  (params (OverlappedComponent :type "PrimitiveComponent Object Reference") (OtherActor :type "Actor Object Reference") (OtherComp :type "PrimitiveComponent Object Reference") (OtherBodyIndex :type Integer) (bFromSweep :type Boolean) (SweepResult :type "HitResult Structure (by ref)"))
  (bind _asbp_player (cast `/Game/Blueprints/BP_Player` OtherActor)
    (:`then`
      (set `self.PlayerCharacter` _asbp_player)
      (set `self.bCanDamage` true))
    (:`CastFailed`
      (`KismetSystemLibrary.PrintString` "Hello" true true (struct :`G` 0.66 :`B` 1.0 :`A` 1.0) 3.0))))

(event `self.Box.OnComponentEndOverlap`
  (params (OverlappedComponent :type "PrimitiveComponent Object Reference") (OtherActor :type "Actor Object Reference") (OtherComp :type "PrimitiveComponent Object Reference") (OtherBodyIndex :type Integer))
  (cast `/Game/Blueprints/BP_Player` OtherActor)
  (set `self.bCanDamage` true))

(fn `UserConstructionScript`)