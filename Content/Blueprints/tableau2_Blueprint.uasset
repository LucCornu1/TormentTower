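; Trigger-volume Blueprint for the second "tableau" that shows an interface widget while the player is nearby.
; When BP_Player enters the Trigger component, it sets TriggerTab2, then creates a BP_interface_tableaux widget and adds it to the viewport.
; When the player leaves, it clears the flag and removes the widget.
; Any other overlapping actor only prints a debug string on entry.
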(event `self.trigger.OnComponentBeginOverlap`
  (params (OverlappedComponent :type "PrimitiveComponent Object Reference") (OtherActor :type "Actor Object Reference") (OtherComp :type "PrimitiveComponent Object Reference") (OtherBodyIndex :type Integer) (bFromSweep :type Boolean) (SweepResult :type "HitResult Structure (by ref)"))
  (cast `/Game/Blueprints/BP_Player` OtherActor
    (:`then`
      (set `self.Trigger_tab2` true)
      (bind _returnvalue (`|CreateWidget` "/Game/Blueprints/widgets/BP_interface_tableaux.BP_interface_tableaux_C"))
      (`UserWidget.AddToViewport` _returnvalue 0))
    (:`CastFailed`
      (`KismetSystemLibrary.PrintString` "Big Nope"))))

(event `self.trigger.OnComponentEndOverlap`
  (params (OverlappedComponent :type "PrimitiveComponent Object Reference") (OtherActor :type "Actor Object Reference") (OtherComp :type "PrimitiveComponent Object Reference") (OtherBodyIndex :type Integer))
  (cast `/Game/Blueprints/BP_Player` OtherActor)
  (set `self.Trigger_tab2` false)
  (`Widget.RemoveFromParent` (stale `self.trigger.OnComponentBeginOverlap` _returnvalue)))

(fn `UserConstructionScript`
  (`parent.UserConstructionScript`))