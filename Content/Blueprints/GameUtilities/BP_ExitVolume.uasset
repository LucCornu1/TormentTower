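; BP_ExitVolume is a level exit trigger that awards points to players who reach it.
; Its box overlap responds to PlayerPaperCharacter actors not yet flagged as exited, ignoring their AttackHitbox component.
; The first arrival earns full Points, and each later scoring overlap halves the value before awarding it.
; Points are added to Player 1's or Player 2's score on BP_GameInstance, chosen by player number.
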(event `self.ReceiveBeginPlay`
  (bind _asbp_game_instance (cast `/Game/Blueprints/GameUtilities/BP_GameInstance` (`GameplayStatics.GetGameInstance`)))
  (set `self.CurrentGameInstance` _asbp_game_instance))

(event `self.BoxComponent.OnComponentBeginOverlap`
  (params (OverlappedComponent :type "PrimitiveComponent Object Reference") (OtherActor :type "Actor Object Reference") (OtherComp :type "PrimitiveComponent Object Reference") (OtherBodyIndex :type Integer) (bFromSweep :type Boolean) (SweepResult :type "HitResult Structure (by ref)"))
  (bind _points (`self.Points`))
  (bind _currentgameinstance (`self.CurrentGameInstance`))
  (bind _currentgameinstance_2 (`self.CurrentGameInstance`))
  (if (!= OtherActor self)
    (bind _asplayer_paper_character (cast `PlayerPaperCharacter` OtherActor))
    (if (`KismetStringLibrary.NotEqual_StrStr` (`KismetSystemLibrary.GetObjectName` OtherComp) "AttackHitbox")
      (if (not (`PlayerPaperCharacter.GetIsExited` _asplayer_paper_character))
        (if (`self.FirstArrived`)
          (set `self.FirstArrived` false)
          (else
            (set `self.Points` (/ (`self.Points`) 2))))
        (if (== (`PlayerPaperCharacter.GetPlayerNumber` _asplayer_paper_character) 0)
          (set `/Game/Blueprints/GameUtilities/BP_GameInstance.Player1Score` (+ (`/Game/Blueprints/GameUtilities/BP_GameInstance.Player1Score` _currentgameinstance_2) _points) _currentgameinstance)
          (else
            (set `/Game/Blueprints/GameUtilities/BP_GameInstance.Player2Score` (+ (`/Game/Blueprints/GameUtilities/BP_GameInstance.Player2Score` _currentgameinstance_2) _points) _currentgameinstance)))))))

(fn `UserConstructionScript`)