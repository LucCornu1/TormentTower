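; BP_Boulder is a Paper2D sprite hazard that starts physics simulation and damages the player.
; When the player character overlaps the Trigger component, the sprite switches on physics simulation.
; Overlaps on the sprite apply damage to any BP_Player.
; The sprite's hit event is empty, and a duplicate damage chain is left disconnected.
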(event `self.Trigger.OnComponentBeginOverlap`
  (params (OverlappedComponent :type "PrimitiveComponent Object Reference") (OtherActor :type "Actor Object Reference") (OtherComp :type "PrimitiveComponent Object Reference") (OtherBodyIndex :type Integer) (bFromSweep :type Boolean) (SweepResult :type "HitResult Structure (by ref)"))
  ;[0.2756 1 0.2323] Activation de la physique à l'entrée de la zone
  (if (== OtherActor (`GameplayStatics.GetPlayerCharacter` 0))
    (`PrimitiveComponent.SetSimulatePhysics` (`self.PaperSprite`) true)))

(event `self.PaperSprite.OnComponentHit`
  (params (HitComponent :type "PrimitiveComponent Object Reference") (OtherActor :type "Actor Object Reference") (OtherComp :type "PrimitiveComponent Object Reference") (NormalImpulse :type "Vector Structure") (Hit :type "HitResult Structure (by ref)"))
  ;[1 0.07396 0.07396] Application de dégâts au contacte d'un joueur
)

(event `self.PaperSprite.OnComponentBeginOverlap`
  (params (OverlappedComponent :type "PrimitiveComponent Object Reference") (OtherActor :type "Actor Object Reference") (OtherComp :type "PrimitiveComponent Object Reference") (OtherBodyIndex :type Integer) (bFromSweep :type Boolean) (SweepResult :type "HitResult Structure (by ref)"))
  (if (!= OtherActor self)
    (bind _asbp_player (cast `/Game/Blueprints/PaperCharacters/BP_Player` OtherActor))
    (`GameplayStatics.ApplyDamage` _asbp_player 1.0 null self)))

(fn `UserConstructionScript`)