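; Mini-game setup Blueprint that spawns the local players and initializes their controls when play begins.
; It reads the player count from BP_GameInstance and matches each index to the PlayerStart tagged with that number.
; There it creates a local player, then spawns, possesses and numbers a BP_PlayerMiniGame.
; Player 0's CustomPlayerController then receives a multiplayer flag and the first two pawns.
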(event `self.ReceiveBeginPlay`
  (bind _players (`self.Players`))
  ;[0.03274 1 0.06022] Apparition des joueurs
  (bind _asbp_game_instance (cast `/Game/Blueprints/GameUtilities/BP_GameInstance` (`GameplayStatics.GetGameInstance`)))
  (set `self.MaxPlayerCount` (`/Game/Blueprints/GameUtilities/BP_GameInstance.NbPlayers` _asbp_game_instance))
  (`self.GetPlayerStartPoints`)
  (`self.SpawnPlayers`)
  ;[0.1315 0.771 1] Initialisation des contrôles
  (bind _ascustom_player_controller (cast `CustomPlayerController` (`GameplayStatics.GetPlayerControllerFromID` 0)))
  (`CustomPlayerController.InitController` _ascustom_player_controller (> (`self.MaxPlayerCount`) 1) (`|GetArrayItem` _players) (`|GetArrayItem` _players 1)))

(fn `GetPlayerStartPoints`
  (bind _outactors (`GameplayStatics.GetAllActorsOfClass` "/Script/Engine.PlayerStart"))
  (set `self.PlayerStartArray` _outactors))

(fn `SpawnPlayers`
  (bind _index (`self.Index`))
  (for _index_2 (range (`self.MaxPlayerCount`))
    (set `self.Index` _index_2)
    (for _array_element (`self.PlayerStartArray`)
      (if (== (`PlayerStart.PlayerStartTag` _array_element) (`KismetStringLibrary.Conv_StringToName` (`KismetStringLibrary.Conv_IntToString` (`self.Index`))))
        (`GameplayStatics.CreatePlayer` (`self.Index`))
        (bind _returnvalue (`|SpawnActorFromClass` "/Game/Blueprints/PaperCharacters/BP_PlayerMini-Game.BP_PlayerMini-Game_C" (`self.GetTransform` _array_element) "AlwaysSpawn" "OverrideRootScale" null null))
        (`Controller.Possess` (`GameplayStatics.GetPlayerControllerFromID` _index) _returnvalue)
        (`PlayerPaperCharacter.SetPlayerNumber` _returnvalue _index)
        (`KismetArrayLibrary.Array_AddUnique` (`self.Players`) _returnvalue)))))

(fn `UserConstructionScript`)