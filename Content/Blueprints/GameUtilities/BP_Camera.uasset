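; BP_Camera is a shared orthographic camera that follows one or two players.
; On BeginPlay it reads the player list from BP_GameModeBase, becomes every PlayerController's view target and starts a fast looping update timer.
; Each update smoothly interpolates the actor toward a point above the lone player or the pair's midpoint.
; With two players, their clamped separation also sets spring arm length and ortho width, zooming to fit.
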(event `self.ReceiveBeginPlay`
  (`KismetSystemLibrary.Delay` 0.001)
  (`self.ClassSetup`)
  (`CameraComponent.SetProjectionMode` (`self.Camera`) "Orthographic")
  (`CameraComponent.SetOrthoWidth` (`self.Camera`) 2000.0)
  (`KismetSystemLibrary.K2_SetTimer` null "UpdateCamera" 0.001 true))

(event `UpdateCamera`
  (switch `int` (`KismetArrayLibrary.Array_Length` (`self.PlayersReference`))
    (:`1`
      (`self.SetCameraPosition_Solo`))
    (:`2`
      (`self.SetArmLength`)
      (`self.SetCameraPosition`))))

(fn `ClassSetup`
  (bind _asbp_game_mode_base (cast `/Game/Blueprints/GameUtilities/BP_GameModeBase` (`GameplayStatics.GetGameMode`)))
  (bind _output_get (set `self.BP_GameMode` _asbp_game_mode_base))
  (set `self.PlayersReference` (`/Game/Blueprints/GameUtilities/BP_GameModeBase.Players` _output_get))
  (bind _outactors (`GameplayStatics.GetAllActorsOfClass` "/Script/Engine.PlayerController"))
  (`PlayerController.SetViewTargetWithBlend` _outactors self 0.0 "VTBlend_Linear" 0.0 false)
  (for (_array_element _array_index) (`self.PlayersReference`)
    (switch `int` _array_index
      (:`0`
        (set `self.Player1` _array_element))
      (:`1`
        (set `self.Player2` _array_element)))))

(fn `SetArmLength`
  (bind _output_get (set `SpringArmComponent.TargetArmLength` (`KismetMathLibrary.FClamp` (`self.GetDistanceTo` (`self.Player1`) (`self.Player2`)) (`self.MinArmLength`) (`self.MaxArmLength`)) (`self.SpringArm`)))
  (`CameraComponent.SetOrthoWidth` (`self.Camera`) (* _output_get 2.0)))

(fn `SetCameraPosition`
  (bind (_returnvalue_x _returnvalue_y _returnvalue_z) (`KismetMathLibrary.BreakVector` (/ (+ (`self.K2_GetActorLocation` (`self.Player1`)) (`self.K2_GetActorLocation` (`self.Player2`))) (`KismetMathLibrary.Conv_IntToDouble` (`KismetArrayLibrary.Array_Length` (`self.PlayersReference`))))))
  (set `self.TargetPos` (`KismetMathLibrary.MakeVector` _returnvalue_x _returnvalue_y (+ _returnvalue_z 100.0)))
  (`self.K2_SetActorLocation` (`KismetMathLibrary.VInterpTo` (`self.CurrentPos`) (`self.TargetPos`) (`GameplayStatics.GetWorldDeltaSeconds`) (`self.InterpSpeed`)))
  (set `self.CurrentPos` (`self.K2_GetActorLocation`)))

(fn `SetCameraPosition_Solo`
  (bind (_returnvalue_x _returnvalue_y _returnvalue_z) (`KismetMathLibrary.BreakVector` (`self.K2_GetActorLocation` (`self.Player1`))))
  (set `self.TargetPos` (`KismetMathLibrary.MakeVector` _returnvalue_x _returnvalue_y (+ _returnvalue_z 100.0)))
  (`self.K2_SetActorLocation` (`KismetMathLibrary.VInterpTo` (`self.CurrentPos`) (`self.TargetPos`) (`GameplayStatics.GetWorldDeltaSeconds`) (`self.InterpSpeed`)))
  (set `self.CurrentPos` (`self.K2_GetActorLocation`)))

(fn `UserConstructionScript`)