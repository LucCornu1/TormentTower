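; Rhythm minigame shooter that fires BP_Projectile_Rythme from its spawn point at a quickening pace while a countdown runs.
; On BeginPlay it creates the MG2 chrono HUD, then after a short delay loops for as long as that widget's counter is above zero.
; Each shot reveals the actor and plays its sprite once, hides it half a second later, and shortens RateOfFire by Acceleration until under a minimum.
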(event `self.ReceiveBeginPlay`
  (bind _spawnpoint (`self.SpawnPoint`))
  (`self.SetActorHiddenInGame` true)
  (`PaperFlipbookComponent.SetLooping` (`self.Sprite`) false)
  (bind _returnvalue (`|CreateWidget` "/Game/Blueprints/widgets/BP_HUD_MG2_Chrono.BP_HUD_MG2_Chrono_C"))
  (`UserWidget.AddToViewport` _returnvalue 0)
  (`KismetSystemLibrary.Delay` 2.0)
  (if (> (`/Game/Blueprints/widgets/BP_HUD_MG2_Chrono.Compte_chrono` _returnvalue) 0) :!label _label
    (`KismetSystemLibrary.Delay` 0.5)
    (`self.SetActorHiddenInGame` true)
    (`KismetSystemLibrary.Delay` (- (`self.RateOfFire`) 0.5))
    (`|SpawnActorFromClass` "/Game/Blueprints/BP_Projectile_Rythme.BP_Projectile_Rythme_C" (`KismetMathLibrary.MakeTransform` (`SceneComponent.K2_GetComponentLocation` _spawnpoint) (`SceneComponent.K2_GetComponentRotation` _spawnpoint) (0.2 0.2 0.2)) "Undefined" "OverrideRootScale" null null)
    (`self.SetActorHiddenInGame` false)
    (`PaperFlipbookComponent.PlayFromStart` (`self.Sprite`))
    (`PaperFlipbookComponent.SetLooping` (`self.Sprite`) false)
    (if (< (`self.RateOfFire`) 0.6)
      (goto _label)
      (else
        (set `self.RateOfFire` (- (`self.RateOfFire`) (`self.Acceleration`)))
        (goto _label)))
    (else
      (`KismetSystemLibrary.PrintString` "Stop Firing")
      (`self.SetActorHiddenInGame` true))))

(fn `UserConstructionScript`)