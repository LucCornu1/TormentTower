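; BP_PlayerMini-Game is a player character Blueprint for a mini-game that handles melee damage through its AttackHitbox.
; Overlap events store the other actor as Ennemi and toggle CanDamage, ignoring itself as a target and toggling only for components not named AttackHitbox.
; Tick applies fixed damage to that single stored target every frame while CanDamage and GetIsAttacking are true, with no once-per-swing guard.
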(event `self.AttackHitbox.OnComponentBeginOverlap`
  (params (OverlappedComponent :type "PrimitiveComponent Object Reference") (OtherActor :type "Actor Object Reference") (OtherComp :type "PrimitiveComponent Object Reference") (OtherBodyIndex :type Integer) (bFromSweep :type Boolean) (SweepResult :type "HitResult Structure (by ref)"))
  ;[1 0.03229 0.03229] Vérification attaque joueur
  (if (!= OtherActor self)
    (set `self.Ennemi` OtherActor)
    (if (`KismetStringLibrary.NotEqual_StrStr` (`KismetSystemLibrary.GetObjectName` OtherComp) "AttackHitbox")
      (set `self.bCanDamage` true))))

(event `self.AttackHitbox.OnComponentEndOverlap`
  (params (OverlappedComponent :type "PrimitiveComponent Object Reference") (OtherActor :type "Actor Object Reference") (OtherComp :type "PrimitiveComponent Object Reference") (OtherBodyIndex :type Integer))
  ;[1 0.03229 0.03229] Vérification attaque joueur
  (if (!= OtherActor self)
    (if (`KismetStringLibrary.NotEqual_StrStr` (`KismetSystemLibrary.GetObjectName` OtherComp) "AttackHitbox")
      (set `self.bCanDamage` false))))

(event `self.ReceiveTick`
  (params (DeltaSeconds :type "Float (single-precision)"))
  ;[1 0.09063 0.09063] Attaque du joueur
  (if (and (`self.bCanDamage`) (`self.GetIsAttacking`))
    (`GameplayStatics.ApplyDamage` (`self.Ennemi`) 1.0 null self)))

(fn `UserConstructionScript`
  (`parent.UserConstructionScript`))