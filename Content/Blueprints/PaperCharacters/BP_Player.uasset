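; Player Paper2D character Blueprint that handles the HUD and melee attack damage.
; On BeginPlay it creates the HUD widget, and OnHitBP refreshes its life bar with current HP.
; AttackHitbox overlaps store another BasePaperCharacter as the target and toggle a CanDamage flag.
; Tick applies damage to that single stored target on every frame that CanDamage and the attacking state are both true.
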(event `self.ReceiveBeginPlay`
  (bind _returnvalue (`|CreateWidget` "/Game/2DTormentTower/HUD/HUD.HUD_C"))
  (bind _output_get (set `self.PlayerHUD` _returnvalue))
  (`UserWidget.AddToViewport` _output_get 0))

(event `self.OnHit_BP`
  (`/Game/2DTormentTower/HUD/HUD.UpdateLifeBar` (`self.PlayerHud`) (`self.GetCurrentHP`)))

(event `self.AttackHitbox.OnComponentBeginOverlap`
  (params (OverlappedComponent :type "PrimitiveComponent Object Reference") (OtherActor :type "Actor Object Reference") (OtherComp :type "PrimitiveComponent Object Reference") (OtherBodyIndex :type Integer) (bFromSweep :type Boolean) (SweepResult :type "HitResult Structure (by ref)"))
  (if (!= OtherActor self)
    (bind _asbase_paper_character (cast `BasePaperCharacter` OtherActor))
    (set `self.Character` _asbase_paper_character)
    (set `self.bCanDamage` true)))

(event `self.AttackHitbox.OnComponentEndOverlap`
  (params (OverlappedComponent :type "PrimitiveComponent Object Reference") (OtherActor :type "Actor Object Reference") (OtherComp :type "PrimitiveComponent Object Reference") (OtherBodyIndex :type Integer))
  (if (!= OtherActor self)
    (cast `BasePaperCharacter` OtherActor)
    (set `self.bCanDamage` false)))

(event `self.ReceiveTick`
  (params (DeltaSeconds :type "Float (single-precision)"))
  (if (and (`self.bCanDamage`) (`self.GetIsAttacking`))
    (`GameplayStatics.ApplyDamage` (`self.Character`) 1.0 null self)))

(fn `UserConstructionScript`)